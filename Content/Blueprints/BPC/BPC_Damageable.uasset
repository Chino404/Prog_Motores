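; Damageable component that gives its owning actor a life value that can be reduced by damage.
; GetDamage subtracts from CurrentLife and fires OnDamaged with the amount.
; When IsAlive finds life at zero or below, it fires OnDeath with the owner and optionally destroys that actor via DestroyOnDeath.
; BeginPlay is empty, as the node copying MaxLife into CurrentLife is unconnected.
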(event EventBeginPlay)

(fn GetDamage
  (params (InDamage :type Float%20%28double-precision%29))
  (Variables|Default|SetCurrentLife (- (Variables|Default|GetCurrentLife) InDamage))
  (Default|CallOnDamaged InDamage)
  (if (not (CallFunction|IsAlive))
    (Default|CallOnDeath (Components|GetOwner))
    (if (Variables|Default|GetDestroyOnDeath)
      (Actor|DestroyActor (Components|GetOwner)))))

(fn IsAlive
  (return (> (Variables|Default|GetCurrentLife) 0.0)))