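; Bear trap actor that immobilizes the third-person character on overlap until released through an interact input.
; Overlap snaps the player to the box's center, disables movement, shows WBP_Interact, enables input on the trap, turns off collision and swaps the material.
; InteractTramp, debounced by a short timer, restores walking and removes the prompt.
; Another timer then re-enables collision, re-arming the trap, and timers reset the material.
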(event OnComponentBeginOverlap(BoxCollision)
  (params (OverlappedComponent :type Primitive%20Component%20Object%20Reference) (OtherActor :type Actor%20Object%20Reference) (OtherComp :type Primitive%20Component%20Object%20Reference) (OtherBodyIndex :type Integer) (bFromSweep :type Boolean) (SweepResult :type Hit%20Result%20Structure%20%28by%20ref%29))
  (bind _asbp_third_person_character (Utilities|Casting|CastToBP_ThirdPersonCharacter OtherActor))
  (CallFunction|AtraparJugador _asbp_third_person_character)
  (Input|EnableInput (Game|GetPlayerController 0))
  (Collision|SetCollisionEnabled (Variables|Components|GetBoxCollision) "NoCollision")
  (Rendering|Material|SetMaterial (Variables|Components|GetTrap) 0 "/Game/Blueprints/MI_BearTrapActive.MI_BearTrapActive"))

(event Custom|Atrapar%20Jugador
  (params (Character :type Character%20Object%20Reference))
  (bind _boxcollision (Variables|Components|GetBoxCollision))
  (bind _returnvalue (Transformation|GetWorldLocation _boxcollision))
  ;[1 1 1] Atrapar al jugador
  (Pawn|Components|CharacterMovement|DisableMovement (Variables|/Script/Engine.Character|GetCharacterMovement Character))
  (Transformation|SetActorLocation Character (Math|Vector|MakeVector (.x _returnvalue) (.y _returnvalue) (.z (Transformation|GetActorLocation Character))) false false)
  (Rendering|Material|SetMaterial (Variables|Components|GetTrap) 0 "/Game/Blueprints/MI_BearTrapDesactive.MI_BearTrapDesactive")
  ;[1 1 1] Mostrar Interfaz
  (bind _returnvalue_2 (UserInterface|CreateWidget "/Game/Widgets/WBP_Interact.WBP_Interact_C"))
  (UserInterface|Viewport|AddtoViewport _returnvalue_2 0))

(event Custom|Abrir%20Trampa
  ;[1 1 1] Abrir Trampa
  (Pawn|Components|CharacterMovement|SetMovementMode (Variables|/Script/Engine.Character|GetCharacterMovement (stale OnComponentBeginOverlap(BoxCollision) _asbp_third_person_character)) "MOVE_Walking" 0)
  ;;[1 1 1] Quitar Interfaz
  (Widget|RemovefromParent (stale Custom|Atrapar%20Jugador _returnvalue_2))
  (Utilities|Time|SetTimerbyEvent (delegate Custom|CustomEvent_0) 1.0))

(event Custom|Interact%20Tramp
  ;[1 1 1] Input para abrir trampa
  (if (not (Variables|Default|GetPresionar))
    (CallFunction|AbrirTrampa)
    (Variables|Default|SetPresionar true)
    (Utilities|Time|SetTimerbyEvent (delegate Custom|CustomEvent) 0.5)))

(event Custom|CustomEvent
  ;[1 1 1] Input para abrir trampa
  (Variables|Default|SetPresionar false)
  (Rendering|Material|SetMaterial (Variables|Components|GetTrap) 0 "/Game/Blueprints/MI_BearTrapDesactive.MI_BearTrapDesactive"))

(event Custom|CustomEvent_0
  ;[1 1 1] Abrir Trampa
  (Collision|SetCollisionEnabled (Variables|Components|GetBoxCollision) "QueryAndPhysics")
  (Rendering|Material|SetMaterial (Variables|Components|GetTrap) 0 "/Game/Blueprints/MI_BearTrapDesactive.MI_BearTrapDesactive"))

(fn ConstructionScript)