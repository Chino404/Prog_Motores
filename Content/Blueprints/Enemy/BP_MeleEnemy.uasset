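; Melee enemy that writes sensed actors to its AI blackboard, clearing the key when sensing fails.
; Punch briefly enables a collider on a timer; its overlaps apply fixed damage to actors with BPC_Damageable.
; Its own BPC_Damageable death event ragdolls the mesh and destroys it after a delay, but AnyDamage destroys it immediately.
; BP_Hit spawning and EnPosicion setters are unconnected.
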(event OnTargetPerceptionUpdated(AIPerception)
  (params (Actor :type Actor%20Object%20Reference) (Stimulus :type AI%20Stimulus%20Structure))
  (AI|Components|Blackboard|SetValueasObject (AI|GetBlackboard (Pawn|GetController)) (Variables|Default|GetKeyName) (Utilities|SelectObject Actor 0 (.bSuccessfullySensed (Utilities|Struct|BreakAIStimulus Stimulus)))))

(event OnDeath(BPC_Damageable)
  (params (KillerActor :type Actor%20Object%20Reference))
  (Physics|SetSimulatePhysics (Variables|Character|GetMesh) true)
  (Utilities|Time|SetTimerbyEvent (delegate Custom|Destroy) 0.5))

(event OnComponentBeginOverlap(Punch_Collider)
  (params (OverlappedComponent :type Primitive%20Component%20Object%20Reference) (OtherActor :type Actor%20Object%20Reference) (OtherComp :type Primitive%20Component%20Object%20Reference) (OtherBodyIndex :type Integer) (bFromSweep :type Boolean) (SweepResult :type Hit%20Result%20Structure%20%28by%20ref%29))
  (for _array_element (Collision|GetOverlappingActors (Variables|Default|GetPunch_Collider) 0 :!class /Script/Engine.PrimitiveComponent)
    (Utilities|IsValid (Actor|GetComponentbyClass _array_element "/Game/ThirdPerson/Blueprints/BPC_Damageable.BPC_Damageable_C")
      (:Is%20Valid
        (Default|GetDamage (Actor|GetComponentbyClass _array_element "/Game/ThirdPerson/Blueprints/BPC_Damageable.BPC_Damageable_C") 1e+01)))))

(event Custom|Punch
  (Collision|SetCollisionEnabled (Variables|Default|GetPunch_Collider) "QueryAndPhysics")
  (Utilities|Time|SetTimerbyEvent (delegate Custom|DesactivarCollision) 0.3))

(event Custom|Destroy
  (Actor|DestroyActor))

(event Custom|DesactivarCollision
  (Collision|SetCollisionEnabled (Variables|Default|GetPunch_Collider) "NoCollision"))

(event Game|Damage|EventAnyDamage
  (params (Damage :type Float%20%28single-precision%29) (DamageType :type Damage%20Type%20Object%20Reference) (InstigatedBy :type Controller%20Object%20Reference) (DamageCauser :type Actor%20Object%20Reference))
  (Actor|DestroyActor self))

(event EventBeginPlay
  (Collision|SetCollisionEnabled (Variables|Default|GetPunch_Collider) "NoCollision"))

(fn ConstructionScript)