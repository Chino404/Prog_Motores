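; Base enemy Blueprint that configures life, skin, materials, AI controller and bullet class from a DT_Eenemies row during construction.
; AI perception writes the sensed actor to a Blackboard key.
; Punch briefly enables a collider that damages BPC_Damageable actors; Shoot aims at the player controller's focal location and spawns a hard-coded BP_Bullet.
; AnyDamage destroys the enemy immediately, while BPC_Damageable death enables mesh physics before delayed destruction.
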(event OnTargetPerceptionUpdated(AIPerception)
  (params (Actor :type Actor%20Object%20Reference) (Stimulus :type AI%20Stimulus%20Structure))
  (AI|Components|Blackboard|SetValueasObject (AI|GetBlackboard (Pawn|GetController)) (Variables|Default|GetKeyName) (Utilities|SelectObject Actor 0 (.bSuccessfullySensed (Utilities|Struct|BreakAIStimulus Stimulus)))))

(event OnDeath(BPC_Damageable)
  (params (KillerActor :type Actor%20Object%20Reference))
  (Physics|SetSimulatePhysics (Variables|Character|GetMesh) true)
  (Utilities|Time|SetTimerbyEvent (delegate Custom|Destroy) 0.5))

(event OnComponentBeginOverlap(Punch_Collider)
  (params (OverlappedComponent :type Primitive%20Component%20Object%20Reference) (OtherActor :type Actor%20Object%20Reference) (OtherComp :type Primitive%20Component%20Object%20Reference) (OtherBodyIndex :type Integer) (bFromSweep :type Boolean) (SweepResult :type Hit%20Result%20Structure%20%28by%20ref%29))
  (for _array_element (Collision|GetOverlappingActors (Variables|Default|GetPunch_Collider) 0 :!class /Script/Engine.PrimitiveComponent)
    (Utilities|IsValid (Actor|GetComponentbyClass _array_element "/Game/ThirdPerson/Blueprints/BPC_Damageable.BPC_Damageable_C")
      (:Is%20Valid
        (Default|GetDamage (Actor|GetComponentbyClass _array_element "/Game/ThirdPerson/Blueprints/BPC_Damageable.BPC_Damageable_C") 1e+01)))))

(event Custom|Shoot
  ;[1 1 1] Rotacion Arrow
  (if (not (Variables|Default|GetIsShooting))
    (Variables|Default|SetIsShooting true)
    (Transformation|SetWorldRotation (Variables|Default|GetPositionPunch) (Math|Rotator|FindLookatRotation (Transformation|GetWorldLocation (Variables|Default|GetPositionPunch)) (Class|PlayerController|GetFocalLocation (Game|GetPlayerController 0))) false false)
    (Variables|Default|SetIsShooting false)
    (Audio|PlaySound2D "/Game/StarterContent/Audio/Sonido-Disparo_Cue.Sonido-Disparo_Cue" 1.0 1.0 0.0 0 0)
    (Game|SpawnActorfromClass "/Game/Blueprints/BP_Bullet.BP_Bullet_C" (Transformation|GetWorldTransform (Variables|Default|GetPositionPunch)) "AlwaysSpawn" "MultiplyWithRoot" 0 0)))

(event Custom|Destroy
  (Actor|DestroyActor))

(event Custom|DesactivarCollision
  ;[1 1 1] Punch
  (Variables|Default|SetIsAttacking false)
  (Collision|SetCollisionEnabled (Variables|Default|GetPunch_Collider) "NoCollision"))

(event Custom|Punch
  ;[1 1 1] Punch
  (if (not (Variables|Default|GetIsAttacking))
    (Collision|SetCollisionEnabled (Variables|Default|GetPunch_Collider) "QueryAndPhysics")
    (Variables|Default|SetIsAttacking true)
    (Utilities|Time|SetTimerbyEvent (delegate Custom|DesactivarCollision) 0.3)))

(event Game|Damage|EventAnyDamage
  (params (Damage :type Float%20%28single-precision%29) (DamageType :type Damage%20Type%20Object%20Reference) (InstigatedBy :type Controller%20Object%20Reference) (DamageCauser :type Actor%20Object%20Reference))
  (Actor|DestroyActor self))

(event EventBeginPlay
  (Collision|SetCollisionEnabled (Variables|Default|GetPunch_Collider) "NoCollision"))

(fn ConstructionScript
  (CallFunction|InitializeEnemy))

(fn InitializeEnemy
  (bind _returnvalue (Utilities|GetDataTableRow "/Game/Blueprints/DataTable/DT_Eenemies.DT_Eenemies" (Variables|Default|GetRow%20Name))
    (:then
      (Variables|Default|SetMax%20Life (.MaxLife (Utilities|Struct|BreakEnemyData _returnvalue)))
      (Variables|/Game/ThirdPerson/Blueprints/BPC_Damageable.BPC_Damageable_C|SetCurrentLife (Variables|Default|GetBPC_Damageable) 0.0)
      (Components|SkeletalMesh|SetSkeletalMeshAsset (Variables|Character|GetMesh) (.Skin (Utilities|Struct|BreakEnemyData _returnvalue)))
      (for (_array_element _array_index) (.Materials (Utilities|Struct|BreakEnemyData _returnvalue))
        (Rendering|Material|SetMaterial (Variables|Character|GetMesh) _array_index _array_element)
        (bind _output_get (Variables|Default|SetAIC (.AIC (Utilities|Struct|BreakEnemyData _returnvalue))))
        (Variables|Default|SetAIControllerClass _output_get)
        (Variables|Default|SetBullet%20Spawn (.BulletSpawn (Utilities|Struct|BreakEnemyData _returnvalue)))))))