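; BP_RangeEnemy is a ranged enemy that fires projectiles at the player and is destroyed by any damage.
; AI perception updates write the sensed actor to a Blackboard key, or clear it when sensing fails.
; Its Shoot event rotates the RotationnBullet component toward the player controller's focal location, spawns BP_Bullet from that transform, plays a shot sound and prints a debug message.
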(event OnTargetPerceptionUpdated(AIPerception)
  (params (Actor :type Actor%20Object%20Reference) (Stimulus :type AI%20Stimulus%20Structure))
  (AI|Components|Blackboard|SetValueasObject (AI|GetBlackboard (Pawn|GetController)) (Variables|Default|GetKeyName) (Utilities|SelectObject Actor 0 (.bSuccessfullySensed (Utilities|Struct|BreakAIStimulus Stimulus)))))

(event Custom|Shoot
  ;[1 1 1] Rotacion Arrow
  (Transformation|SetWorldRotation (Variables|Default|GetRotationnBullet) (Math|Rotator|FindLookatRotation (Transformation|GetWorldLocation (Variables|Default|GetRotationnBullet)) (Class|PlayerController|GetFocalLocation (Game|GetPlayerController 0))) false false)
  (Audio|PlaySound2D "/Game/StarterContent/Audio/Sonido-Disparo_Cue.Sonido-Disparo_Cue" 1.0 1.0 0.0 0 0)
  (Game|SpawnActorfromClass "/Game/Blueprints/BP_Bullet.BP_Bullet_C" (Transformation|GetWorldTransform (Variables|Default|GetRotationnBullet)) "AlwaysSpawn" "MultiplyWithRoot" 0 0)
  (Development|PrintString "Disparo" true true "(R=0.000000,G=0.660000,B=1.000000,A=1.000000)" 3e+01))

(event Game|Damage|EventAnyDamage
  (params (Damage :type Float%20%28single-precision%29) (DamageType :type Damage%20Type%20Object%20Reference) (InstigatedBy :type Controller%20Object%20Reference) (DamageCauser :type Actor%20Object%20Reference))
  (Actor|DestroyActor self))

(fn ConstructionScript)