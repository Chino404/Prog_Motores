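; BP_Hit is a short-lived punch hitbox actor that deals fixed damage to damageable actors it overlaps.
; A timer set on BeginPlay destroys the actor after a fraction of a second.
; On overlap, it loops through actors overlapping its Hit component, calls GetDamage on those with a BPC_Damageable component, and destroys Hit upon damaging.
; An older BP_MeleEnemy cast using ApplyDamage remains disconnected.
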(event Custom|Desactivar%20Punch
  (Actor|DestroyActor))

(event EventBeginPlay
  (Utilities|Time|SetTimerbyEvent (delegate Custom|Desactivar%20Punch) 0.2))

(event Collision|EventActorBeginOverlap
  (params (OtherActor :type Actor%20Object%20Reference))
  (for _array_element (Collision|GetOverlappingActors (Variables|Default|GetHit) 0 :!class /Script/Engine.PrimitiveComponent)
    (Utilities|IsValid (Actor|GetComponentbyClass _array_element "/Game/ThirdPerson/Blueprints/BPC_Damageable.BPC_Damageable_C")
      (:Is%20Valid
        (Default|GetDamage (Actor|GetComponentbyClass _array_element "/Game/ThirdPerson/Blueprints/BPC_Damageable.BPC_Damageable_C") 1e+01)
        (Components|DestroyComponent (Variables|Default|GetHit))))))

(fn ConstructionScript)