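; BP_GI, likely the Game Instance, saves and loads the player's position and current level through a BP_SaveGame slot.
; CargarPartida stores the saved transform, opens the saved level, then moves the pawn there after a short timer via MoverAlJugador.
; GuardarPartida writes pawn transform and level name, creating the save object if no slot exists.
; With an existing slot, it edits the loaded object but saves the SGR variable instead.
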(event Custom|Guardar%20Partida
  (bind _returnvalue (Game|Player|GetPlayerPawn 0))
  (bind _slot_name (Variables|Default|GetSlot%20Name))
  (bind _returnvalue_2 (Transformation|GetActorTransform _returnvalue))
  (bind _returnvalue_3 (SaveGame|DoesSaveGameExist (Variables|Default|GetSlot%20Name)))
  (if _returnvalue_3
    (bind _returnvalue_4 (SaveGame|LoadGamefromSlot (Variables|Default|GetSlot%20Name)))
    (bind _asbp_save_game (Utilities|Casting|CastToBP_SaveGame _returnvalue_4))
    (Variables|/Game/Blueprints/WBP/BP_SaveGame.BP_SaveGame_C|SetCharacterPosition _asbp_save_game _returnvalue_2)
    (bind _returnvalue_5 (Game|GetCurrentLevelName true))
    (Variables|/Game/Blueprints/WBP/BP_SaveGame.BP_SaveGame_C|SetLevel _asbp_save_game _returnvalue_5)
    (SaveGame|SaveGametoSlot (Variables|Default|GetSGR) _slot_name)
    (else
      (bind _returnvalue_6 (SaveGame|CreateSaveGameObject "/Game/Blueprints/WBP/BP_SaveGame.BP_SaveGame_C"))
      (bind _output_get (Variables|Default|SetSGR _returnvalue_6))
      (Variables|/Game/Blueprints/WBP/BP_SaveGame.BP_SaveGame_C|SetCharacterPosition _output_get _returnvalue_2)
      (bind _returnvalue_7 (Game|GetCurrentLevelName true))
      (Variables|/Game/Blueprints/WBP/BP_SaveGame.BP_SaveGame_C|SetLevel _returnvalue_6 _returnvalue_7)
      (SaveGame|SaveGametoSlot (Variables|Default|GetSGR) _slot_name))))

(event Custom|Cargar%20Partida
  (bind _returnvalue (SaveGame|LoadGamefromSlot (Variables|Default|GetSlot%20Name)))
  (bind _asbp_save_game (Utilities|Casting|CastToBP_SaveGame _returnvalue))
  (bind _output_get (Variables|Default|SetPosicionJugador (Variables|/Game/Blueprints/WBP/BP_SaveGame.BP_SaveGame_C|GetCharacterPosition _asbp_save_game)))
  (Game|OpenLevel(byName) (Utilities|String|StringToName (Variables|/Game/Blueprints/WBP/BP_SaveGame.BP_SaveGame_C|GetLevel _asbp_save_game)))
  (Utilities|Time|SetTimerbyEvent (delegate Custom|Mover%20al%20Jugador) 0.2))

(event Custom|Mover%20al%20Jugador
  (Transformation|SetActorTransform (Game|Player|GetPlayerPawn 0) (stale Custom|Cargar%20Partida _output_get)))