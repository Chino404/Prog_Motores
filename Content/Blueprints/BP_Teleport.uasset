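; BP_Teleport is an interactable pad that sends the third-person character to a linked Destino teleporter when E is pressed.
; Overlapping its Collision enables input on the actor and shows the WBP_Interact prompt; leaving disables input and removes it.
; The destination pad's Recibiendo flag is raised briefly around the teleport, blocking an immediate return trip before the player lands slightly above it.
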(event OnComponentBeginOverlap(Collision)
  (params (OverlappedComponent :type Primitive%20Component%20Object%20Reference) (OtherActor :type Actor%20Object%20Reference) (OtherComp :type Primitive%20Component%20Object%20Reference) (OtherBodyIndex :type Integer) (bFromSweep :type Boolean) (SweepResult :type Hit%20Result%20Structure%20%28by%20ref%29))
  ;[1 1 1] Entre en el Trigger
  (bind _asbp_third_person_character (Utilities|Casting|CastToBP_ThirdPersonCharacter OtherActor))
  ;[1 1 1] Activar Input
  (Input|EnableInput (Game|GetPlayerController 0))
  ;[1 1 1] Mostrar Interfaz
  (bind _returnvalue (UserInterface|CreateWidget "/Game/Widgets/WBP_Interact.WBP_Interact_C"))
  (UserInterface|Viewport|AddtoViewport _returnvalue 0))

(event OnComponentEndOverlap(Collision)
  (params (OverlappedComponent :type Primitive%20Component%20Object%20Reference) (OtherActor :type Actor%20Object%20Reference) (OtherComp :type Primitive%20Component%20Object%20Reference) (OtherBodyIndex :type Integer))
  ;[1 1 1] Sali del Tirgger
  (Utilities|Casting|CastToBP_ThirdPersonCharacter OtherActor)
  ;[1 1 1] Desactivar Input
  (Input|DisableInput (Game|GetPlayerController 0))
  ;[1 1 1] Quitar Interfaz
  (Widget|RemovefromParent (stale OnComponentBeginOverlap(Collision) _returnvalue)))

(event Input|KeyboardEvents|E
  (params (Key :type Key%20Structure :default "None"))
  ;[1 1 1] Teletransportarme
  (:Pressed
    (if (not (Variables|Default|GetRecibiendo))
      (bind _asbp_teleport (Utilities|Casting|CastToBP_Teleport (Variables|Default|GetDestino)))
      (Variables|BP_Teleport_C|SetRecibiendo _asbp_teleport true)
      (Transformation|Teleport (stale OnComponentBeginOverlap(Collision) _asbp_third_person_character) (+ (Transformation|GetActorLocation _asbp_teleport) "0.000000,0.000000,50.000000") "0, 0, 0")
      (Utilities|FlowControl|Delay 0.5)
      (Variables|BP_Teleport_C|SetRecibiendo _asbp_teleport false))))

(fn ConstructionScript)