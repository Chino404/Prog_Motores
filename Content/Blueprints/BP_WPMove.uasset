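; BP_WPMove is a lethal moving actor that shuttles between two referenced points and applies massive damage to any actor that overlaps it.
; On BeginPlay, a timeline lerps its location from InitialPoint to FinalPoint without sweep, then alternates reversing and replaying for an endless ping-pong.
; The timeline play rate is the inverse of Velocity, so a higher Velocity value gives slower movement.
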(event EventBeginPlay
  (Components|Timeline|SetPlayRate (Variables|Default|GetMOVETIMELINE) (/ 1.0 (Variables|Default|GetVelocity)))
  (bind (_direction _delta_time) (Timeline|MoveTimeline Play)
    (:Update
      (Transformation|SetActorLocation (Math|Vector|Lerp(Vector) (Transformation|GetActorLocation (Variables|Default|GetInitial%20point)) (Transformation|GetActorLocation (Variables|Default|GetFinal%20Point)) _delta_time) false false))
    (:Finished
      (switch Utilities|FlowControl|Switch|SwitchonETimelineDirection _direction
        (:Forward
          (Timeline|MoveTimeline Reverse))
        (:Backward
          (Timeline|MoveTimeline PlayFromStart))))))

(event Collision|EventActorBeginOverlap
  (params (OtherActor :type Actor%20Object%20Reference))
  (Game|Damage|ApplyDamage OtherActor 1e+05 0 0))

(fn ConstructionScript)

(fn NewFunction)