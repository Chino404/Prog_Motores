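; Stationary shooter turret that fires BP_Bullet when it sees the third-person player character and is destroyed by any damage.
; PawnSensing triggers a delayed sequence that switches the turret meshes to an active material as a warning, then spawns the bullet at the Arrow's transform and restores the material.
; An unconnected copy of the firing sequence that rotates the Arrow toward the player never runs, so the live logic does not aim.
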(event OnSeePawn(PawnSensing)
  (params (Pawn :type Pawn%20Object%20Reference))
  (Utilities|Casting|CastToBP_ThirdPersonCharacter Pawn)
  (Utilities|FlowControl|Delay 1.0)
  (Rendering|Material|SetMaterial (Variables|Default|GetTorrata%20base) 0 "/Game/Blueprints/MI_ActiveShooter.MI_ActiveShooter")
  (Utilities|FlowControl|Delay 1.0)
  (Game|SpawnActorfromClass "/Game/Blueprints/BP_Bullet.BP_Bullet_C" (Transformation|GetWorldTransform (Variables|Default|GetArrow)) "AlwaysSpawn" "MultiplyWithRoot" 0 0)
  (Rendering|Material|SetMaterial (Variables|Default|GetTorrata%20base) 0 "/Game/StarterContent/Materials/M_AssetPlatform.M_AssetPlatform"))

(event Game|Damage|EventAnyDamage
  (params (Damage :type Float%20%28single-precision%29) (DamageType :type Damage%20Type%20Object%20Reference) (InstigatedBy :type Controller%20Object%20Reference) (DamageCauser :type Actor%20Object%20Reference))
  (Actor|DestroyActor self))

(fn ConstructionScript)